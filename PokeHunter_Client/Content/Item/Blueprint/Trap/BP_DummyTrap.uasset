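; BP_DummyTrap is a decoy trap actor that emits a howl and can explode for area damage.
; Three seconds after BeginPlay it plays the howling sound and reports a noise event at its location, which AI hearing can pick up.
; A separate Explode event, not triggered within this Blueprint, applies radial damage with a custom prevention channel, then destroys the actor.
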(event EventBeginPlay
  (bind _returnvalue (Transformation|GetActorLocation))
  (bind _self self)
  (Utilities|FlowControl|Delay 3.0)
  (Audio|PlaySoundatLocation "/Game/Partner/Sound/Sound_Howling.Sound_Howling" _returnvalue "0, 0, 0" 1.0 1.0 0.0 0 0 _self 0)
  (Class|AISenseHearing|ReportNoiseEvent _returnvalue 1.0 _self 0.0 "None"))

(event Collision|EventActorBeginOverlap
  (params (OtherActor :type Actor%20Object%20Reference)))

(event EventTick
  (params (DeltaSeconds :type Float%20%28single-precision%29)))

(event EventExplode
  (Game|Damage|ApplyRadialDamage (Variables|Default|GetDamage) (Transformation|GetActorLocation) (Variables|Default|GetExplosionRadus) "/Script/Engine.DamageType" 0 0 0 false "ECC_GameTraceChannel8")
  (Actor|DestroyActor))

(fn ConstructionScript)