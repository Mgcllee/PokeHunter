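; Behavior tree task that moves an Enemy to a random wander point around its base location.
; On execute it picks a random reachable point within the enemy's MoveRange of BaseLocation and runs AI MoveTo to it.
; On arrival it writes a random float between one and five seconds to a blackboard key, likely a wait time, and succeeds; a failed move fails the task.
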(event EventReceiveExecuteAI
  (params (OwnerController :type AI%20Controller%20Object%20Reference) (ControlledPawn :type Pawn%20Object%20Reference))
  (bind _asenemy (Utilities|Casting|CastToEnemy ControlledPawn))
  (AI|AIMoveTo _asenemy (.RandomLocation (AI|Navigation|GetRandomReachablePointinRadius (Variables|/Script/PokeHunter.Enemy|GetBaseLocation _asenemy) (Variables|/Script/PokeHunter.Enemy|GetMoveRange _asenemy) 0 0)) 0 5.0 false
    (:OnSuccess
      (AI|Components|Blackboard|SetValueasFloat (AI|GetBlackboard OwnerController) (Variables|Default|GetKey%20Name) (Math|Random|RandomFloatinRange 1.0 5.0))
      (AI|BehaviorTree|FinishExecute true))
    (:OnFail
      (AI|BehaviorTree|FinishExecute false))))