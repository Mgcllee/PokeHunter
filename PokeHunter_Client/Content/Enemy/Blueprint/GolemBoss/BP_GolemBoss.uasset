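; Golem boss with breakable arms and hands, a grab-and-throw attack and on-screen damage numbers.
; DestroyPart detaches meshes as physics debris, attaching damage fields to main broken pieces and flagging lost hands.
; Breaking the right shoulder replaces a still-intact forearm with a BP_PartEnemy_2 spawned through an RPC.
; LaunchGrabbedTargets damages held targets and throws them in a forward fan; SpawnGroundEffect line-traces down to place crack-wave VFX.
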(event Custom|ShowDamage
  (params (DamageAmount :type Float%20%28single-precision%29) (HitLoc :type Vector))
  (bind _returnvalue (UserInterface|CreateWidget "/Game/UI/WBP_DamageDisplay.WBP_DamageDisplay_C" 0 DamageAmount HitLoc))
  (bind _aswbp_damage_display (Utilities|Casting|CastToWBP_DamageDisplay _returnvalue))
  (UserInterface|Viewport|AddtoViewport _aswbp_damage_display 0))

(event Custom|RPC_SpawnPartMob
  (params (Trans :type Transform) (Target :type Pawn%20Object%20Reference))
  (Game|SpawnActorfromClass "/Game/Enemy/Blueprint/PartEnemy/BP_PartEnemy_2.BP_PartEnemy_2_C" (Math|Transform|MakeTransform (.location Trans) "0, 0, 0" (.scale Trans)) "AlwaysSpawn" "MultiplyWithRoot" 0 0))

(event Custom|RPC_SpawnField
  (params (LocVec :type Vector))
  (Game|SpawnActorfromClass "/Game/Enemy/Blueprint/GolemBoss/B_DamageField.B_DamageField_C" (Math|Transform|MakeTransform LocVec "0, 0, 0" "1.000000,1.000000,1.000000") "AlwaysSpawn" "MultiplyWithRoot" 0 0))

(event Custom|RPC_SpawnDamageField
  (params (NewParam :type Vector) (Parent :type Scene%20Component%20Object%20Reference))
  (bind _returnvalue (Game|SpawnActorfromClass "/Game/Enemy/Blueprint/GolemBoss/B_DamageField.B_DamageField_C" (Math|Transform|MakeTransform NewParam "0, 0, 0" "1.000000,1.000000,1.000000") "AlwaysSpawn" "MultiplyWithRoot" 0 0))
  (Transformation|AttachComponentToComponent _returnvalue Parent "None" "SnapToTarget" "SnapToTarget" "SnapToTarget" true))

(event EventBeginPlay
  (EventDispatchers|BindEventtoOnDamage (delegate Custom|ShowDamage)))

(event Collision|EventActorBeginOverlap
  (params (OtherActor :type Actor%20Object%20Reference)))

(event EventTick
  (params (DeltaSeconds :type Float%20%28single-precision%29)))

(event EventDestroyPart
  (params (PartName :type Name%20%28by%20ref%29 :default "None"))
  (bind _rightforearm (Variables|Default|GetRightForearm))
  ;[1 1 1] Destroy Part
  (Audio|PlaySoundatLocation "/Game/Sound/SE/Golem_destruction0.Golem_destruction0" (Transformation|GetActorLocation) "0, 0, 0" 1.0 1.0 0.0 "/Game/Enemy/Blueprint/GolemBoss/BP_GolemSound.BP_GolemSound" 0 0 0)
  (switch name PartName
    (:LeftArm
      (CallFunction|DestroyPartMesh (Variables|Default|GetLeftShoulder))
      (CallFunction|DetachUnderGeometry (Variables|Default|GetLeftHand))
      (CallFunction|DestroyLeftHand)
      (CallFunction|DetachLeafPart (Variables|Default|GetLeftUpperArmMesh))
      (Variables|Default|SetbLoseLeftHand true))
    (:LeftHand
      (CallFunction|DestroyPartMesh (Variables|Default|GetLeftHand))
      (CallFunction|DestroyLeftHand)
      (Variables|Default|SetbLoseLeftHand true))
    (:RightHand
      (CallFunction|DestroyPartMesh (Variables|Default|GetRightHand))
      (CallFunction|DestroyRightHand)
      (Variables|Default|SetbLoseRightHand true))
    (:RightArm
      (CallFunction|DestroyPartMesh (Variables|Default|GetRightForearm))
      (CallFunction|DetachUnderGeometry (Variables|Default|GetRightHand))
      (CallFunction|DestroyRightHand)
      (Variables|Default|SetbLoseRightHand true)
      (Variables|Default|SetbDestroyedPart true))
    (:RightShoulder
      (CallFunction|DestroyPartMesh (Variables|Default|GetRightShoulder))
      (if (Variables|Default|GetbDestroyedPart)
        _
        (else
          (CallFunction|RPCSpawnPartMob (Transformation|GetWorldTransform _rightforearm))
          (Components|DestroyComponent _rightforearm)))
      (CallFunction|DetachLeafPart (Variables|Default|GetRightUpperArmMesh))
      (CallFunction|DetachUnderGeometry (Variables|Default|GetRightHand))
      (CallFunction|DestroyRightHand)
      (Variables|Default|SetbLoseRightHand true))))

(fn ConstructionScript)

(fn DestroyPartMesh
  (params (NewParam :type Geometry%20Collection%20Component%20Object%20Reference))
  (Physics|SetSimulatePhysics NewParam true)
  (Collision|SetCollisionEnabled NewParam "QueryAndPhysics")
  (Collision|SetCollisionProfileName NewParam "BlockAll" true :!class /Script/Engine.PrimitiveComponent)
  (Transformation|DetachFromComponent NewParam "KeepWorld" "KeepWorld" "KeepWorld" true)
  (CallFunction|RPCSpawnDamageField (Transformation|GetWorldLocation NewParam) NewParam))

(fn DestroyRightHand
  (Utilities|FlowControl|Sequence
    (:then_0
      (CallFunction|DetachLeafPart (Variables|Default|GetRightFinger0Mesh)))
    (:then_1
      (CallFunction|DetachLeafPart (Variables|Default|GetRightFinger1Mesh)))
    (:then_2
      (CallFunction|DetachLeafPart (Variables|Default|GetRightFinger01Mesh)))
    (:then_3
      (CallFunction|DetachLeafPart (Variables|Default|GetRightFinger11Mesh)))
    (:then_4
      (CallFunction|DetachLeafPart (Variables|Default|GetRightFinger2Mesh)))
    (:then_5
      (CallFunction|DetachLeafPart (Variables|Default|GetRightFinger21Mesh)))
    (:then_6
      (CallFunction|DetachLeafPart (Variables|Default|GetRightFinger3Mesh)))
    (:then_7
      (CallFunction|DetachLeafPart (Variables|Default|GetRightFinger31Mesh)))))

(fn DetachLeafPart
  (params (LeafPart :type Static%20Mesh%20Component%20Object%20Reference))
  (Physics|SetSimulatePhysics LeafPart true)
  (Transformation|DetachFromComponent LeafPart "KeepWorld" "KeepWorld" "KeepWorld" true)
  (Collision|SetCollisionObjectType LeafPart "ECC_Destructible")
  (Collision|SetCollisionEnabled LeafPart "QueryAndPhysics"))

(fn DestroyLeftHand
  (Utilities|FlowControl|Sequence
    (:then_0
      (CallFunction|DetachLeafPart (Variables|Default|GetLeftFinger0Mesh)))
    (:then_1
      (CallFunction|DetachLeafPart (Variables|Default|GetLeftFinger01Mesh)))
    (:then_2
      (CallFunction|DetachLeafPart (Variables|Default|GetLeftFinger1Mesh)))
    (:then_3
      (CallFunction|DetachLeafPart (Variables|Default|GetLeftFinger11Mesh)))
    (:then_4
      (CallFunction|DetachLeafPart (Variables|Default|GetLeftFinger2Mesh)))
    (:then_5
      (CallFunction|DetachLeafPart (Variables|Default|GetLeftFinger21Mesh)))
    (:then_6
      (CallFunction|DetachLeafPart (Variables|Default|GetLeftFinger3Mesh)))
    (:then_7
      (CallFunction|DetachLeafPart (Variables|Default|GetLeftFinger31Mesh)))))

(fn DetachUnderGeometry
  (params (NewParam :type Geometry%20Collection%20Component%20Object%20Reference))
  (Physics|SetSimulatePhysics NewParam true)
  (Collision|SetCollisionEnabled NewParam "QueryAndPhysics")
  (Collision|SetCollisionProfileName NewParam "Pawn" true :!class /Script/Engine.PrimitiveComponent)
  (Transformation|DetachFromComponent NewParam "KeepWorld" "KeepWorld" "KeepWorld" true))

(fn LaunchGrabbedTargets
  (bind _returnvalue (Transformation|GetActorLocation))
  (bind _returnvalue_2 (Transformation|GetActorForwardVector))
  (bind _grabbedtargets (Variables|Default|GetGrabbedTargets))
  (bind _launchtargetgap (Variables|Default|GetLaunchTargetGap))
  (bind _returnvalue_3 (Utilities|Array|Length _grabbedtargets))
  (bind _returnvalue_4 (+ _returnvalue_2 "0.000000,0.000000,1.000000"))
  (bind _returnvalue_5 (+ _returnvalue _returnvalue_4))
  (bind _returnvalue_6 (- _returnvalue_5 _returnvalue))
  (for (_array_element _array_index) _grabbedtargets
    (Utilities|IsValid _array_element
      (:Is%20Valid
        (Game|Damage|ApplyDamage _array_element 3e+01 0 self "/Script/Engine.DamageType")
        (Transformation|DetachFromActor _array_element "KeepWorld" "KeepWorld" "KeepWorld")
        (Utilities|Casting|CastToPartner _array_element
          (:then
            (Transformation|SetActorRotation _array_element (Math|Rotator|MakeRotator 0.0 0.0 (.yaw (Pawn|GetControlRotation _array_element :!class /Script/Engine.Pawn)))))
          (:CastFailed
            (Transformation|SetActorRotation _array_element)))
        (if (== (Math|Integer|%(Integer) _returnvalue_3 2) 0)
          (Character|LaunchCharacter _array_element (* (Math|Vector|RotateVector _returnvalue_6 (Math|Rotator|MakeRotator 0.0 0.0 (+ (Math|Conversions|ToFloat(Integer) (+ (/ _launchtargetgap -2) (/ (- _returnvalue_3 1) -2))) (* _launchtargetgap _array_index)))) 1e+03) false false)
          (else
            (Character|LaunchCharacter _array_element (* (Math|Vector|RotateVector _returnvalue_6 (Math|Rotator|MakeRotator 0.0 0.0 (+ (* _launchtargetgap (/ _returnvalue_3 -2)) (* _launchtargetgap _array_index)))) 1e+03) false false)))
        (Class|EnemyInteractInterface|InteractGrabAttack(Message) _array_element))))
  (Utilities|Array|Clear _grabbedtargets))

(fn SpawnGroundEffect
  (params (TargetLoc :type Vector))
  (bind _outhit (Collision|LineTraceByChannel TargetLoc (+ TargetLoc "0.000000,0.000000,-1000.000000") "TraceTypeQuery1" false 0 "None"))
  (Niagara|SpawnSystematLocation "/Game/VFXs/VFX_Quake/VFX_CrackWave.VFX_CrackWave" (.location _outhit) "0, 0, 0" "5.000000,5.000000,5.000000"))

(fn Grabbed
  (for _array_element (Variables|Default|GetGrabbedTargets)
    (bind _ashunter (Utilities|Casting|CastToHunter _array_element))
    (Variables|/Script/PokeHunter.Hunter|SetbGrabbed _ashunter true)))