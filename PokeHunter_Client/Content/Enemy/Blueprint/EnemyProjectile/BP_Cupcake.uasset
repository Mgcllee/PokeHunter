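; BP_Cupcake is an enemy projectile actor that moves vertically in three phases: rise, hold, then descend and vanish.
; Tick raises it by UpSpeed while Active, tracking distance in Legngth and clearing Active at a fixed height.
; It then counts LifeTime down, lowers itself by DownSpeed, and destroys itself as the tracked distance runs out.
; The file contains no collision or damage logic.
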(event EventBeginPlay)

(event Collision|EventActorBeginOverlap
  (params (OtherActor :type Actor%20Object%20Reference)))

(event EventTick
  (params (DeltaSeconds :type Float%20%28single-precision%29))
  (bind _upspeed (Variables|Default|GetUpSpeed))
  (bind _downspeed (Variables|Default|GetDownSpeed))
  (bind _returnvalue (* DeltaSeconds _downspeed))
  (bind _returnvalue_2 (* DeltaSeconds _upspeed))
  (bind _returnvalue_3 (* _returnvalue -1.0))
  (if (Variables|Default|GetActive)
    (Transformation|AddActorWorldOffset (Math|Vector|MakeVector 0.0 0.0 _returnvalue_2))
    (bind _output_get (Variables|Default|SetLegngth (+ _returnvalue_2 (Variables|Default|GetLegngth))))
    (if (>= _output_get 5e+02)
      (Variables|Default|SetActive false))
    (elif (<= (Variables|Default|GetLifeTime) 0.0)
      (Transformation|AddActorWorldOffset (Math|Vector|MakeVector 0.0 0.0 _returnvalue_3))
      (Variables|Default|SetLegngth (+ _returnvalue_3 (Variables|Default|GetLegngth)))
      (if (<= (+ _returnvalue_3 (Variables|Default|GetLegngth)) 0.0)
        (Actor|DestroyActor))
      (else
        (Variables|Default|SetLifeTime (- (Variables|Default|GetLifeTime) DeltaSeconds))))))

(fn ConstructionScript)