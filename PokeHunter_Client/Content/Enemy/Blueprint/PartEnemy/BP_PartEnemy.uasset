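; Enemy part character that damages actors overlapping its attack box and shows incoming damage in an on-screen widget.
; It starts in Falling movement and drives its mesh transform from Tick through Server and Multi events.
; While Trans is set, the mesh snaps to TargetRot at a lowered offset; otherwise it takes an offset control rotation and disables Tick.
; Trans and TargetRot have empty OnRep handlers.
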(event OnComponentBeginOverlap(AttackBox)
  (params (OverlappedComponent :type Primitive%20Component%20Object%20Reference) (OtherActor :type Actor%20Object%20Reference) (OtherComp :type Primitive%20Component%20Object%20Reference) (OtherBodyIndex :type Integer) (bFromSweep :type Boolean) (SweepResult :type Hit%20Result%20Structure%20%28by%20ref%29))
  ;[1 1 1] Attack
  (Game|Damage|ApplyDamage OtherActor (Variables|Default|GetAttackDamage) 0 self))

(event Custom|ShowDamage
  (params (DamageAmount :type Float%20%28single-precision%29) (HitLoc :type Vector))
  ;[1 1 1] BeginPlay Evnet
  (bind _returnvalue (UserInterface|CreateWidget "/Game/UI/WBP_DamageDisplay.WBP_DamageDisplay_C" 0 DamageAmount HitLoc))
  (UserInterface|Viewport|AddtoViewport _returnvalue 0))

(event Custom|ServerPartTransform
  (params (NewParam :type Skinned%20Mesh%20Component%20Object%20Reference))
  (CallFunction|MultiPartTransform NewParam))

(event Custom|MultiPartTransform
  (params (NewParam :type Skinned%20Mesh%20Component%20Object%20Reference))
  (if (Variables|Default|GetTrans)
    (Transformation|SetRelativeTransform (Variables|Character|GetMesh) (Math|Transform|Lerp(Transform) (Math|Transform|MakeTransform (Variables|Default|GettempVec) (Variables|Default|GettempRot) "1.000000,1.000000,1.000000") (Math|Transform|MakeTransform "0.000000,0.000000,-30.000000" (Variables|Default|GetTargetRot) "1.000000,1.000000,1.000000") 1.0) false false)
    (else
      ;[1 1 1] 코멘트
      (Transformation|SetWorldRotation NewParam (Math|Rotator|CombineRotators (Pawn|GetControlRotation :!class /Script/Engine.Pawn) "0.000000,-90.000000,0.000000") false false)
      (Actor|Tick|SetActorTickEnabled false))))

(event EventBeginPlay
  ;[1 1 1] BeginPlay Evnet
  (Pawn|Components|CharacterMovement|SetMovementMode (Variables|Character|GetCharacterMovement) "MOVE_Falling" 0)
  (EventDispatchers|BindEventtoOnDamage (delegate Custom|ShowDamage)))

(event EventTick
  (params (DeltaSeconds :type Float%20%28single-precision%29))
  (CallFunction|ServerPartTransform (Variables|Character|GetMesh)))

(fn ConstructionScript)

(fn OnRepTrans)

(fn OnRepTargetRot)