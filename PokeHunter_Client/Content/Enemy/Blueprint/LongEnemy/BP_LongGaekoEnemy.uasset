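; BP_LongGaekoEnemy is an enemy character Blueprint that adds damage feedback and blast knockback.
; On BeginPlay it binds ShowDamage to OnDamage, spawning a WBP_DamageDisplay viewport widget with the damage amount and hit location.
; RadialDamage launches the character directly away from the damage origin at a fixed speed, overriding its current velocity.
; The construction script stores the actor's location as BaseLocation, which this file does not otherwise use.
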(event Custom|ShowDamage
  (params (DamageAmount :type Float%20%28single-precision%29) (HitLoc :type Vector))
  (bind _returnvalue (UserInterface|CreateWidget "/Game/UI/WBP_DamageDisplay.WBP_DamageDisplay_C" 0 DamageAmount HitLoc))
  (bind _aswbp_damage_display (Utilities|Casting|CastToWBP_DamageDisplay _returnvalue))
  (UserInterface|Viewport|AddtoViewport _aswbp_damage_display 0))

(event EventBeginPlay
  (EventDispatchers|BindEventtoOnDamage (delegate Custom|ShowDamage)))

(event Game|Damage|EventRadialDamage
  (params (DamageReceived :type Float%20%28single-precision%29) (DamageType :type Damage%20Type%20Object%20Reference) (Origin :type Vector :default "0, 0, 0") (HitInfo :type Hit%20Result%20Structure%20%28by%20ref%29) (InstigatedBy :type Controller%20Object%20Reference) (DamageCauser :type Actor%20Object%20Reference))
  (Character|LaunchCharacter (* (Math|Vector|Normalize (- (Transformation|GetActorLocation) Origin)) 1e+03) true true))

(fn ConstructionScript
  (Variables|Default|SetBaseLocation (Transformation|GetActorLocation)))