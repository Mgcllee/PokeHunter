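; NewHunter is the player hunter character Blueprint, handling UI input, music and combat reactions on top of inherited state.
; Input drives pause, inventory and quick slots through WBP_MainUI, while BGM follows level, boss and ending events with adjustable volume.
; Radial damage and earthquakes launch the character, and a K-key cheat damages every GolemBoss via server/multicast-named events.
; Partner mode projects a surface-aligned cursor with click pings; EndPlay saves inventory to the GameInstance.
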(event Custom|Multicast_EndGame
  ;[1 1 1] End Game BGM
  (Audio|Components|Audio|SetSound (Variables|Default|GetBGM) "/Game/Sound/BGM/BGM_Complete0.BGM_Complete0"))

(event Custom|AllKill_Server
  ;[1 1 1] Command Kill ALL
  (bind _outactors (Actor|GetAllActorsOfClass "/Script/PokeHunter.GolemBoss"))
  (for _array_element _outactors
    (CallFunction|AllKillMulti _array_element)))

(event Custom|AllKillMulti
  (params (NewParam :type Enemy%20Object%20Reference))
  ;[1 1 1] Command Kill ALL
  (Game|Damage|ApplyDamage NewParam 5e+06 0 0))

(event Custom|Multicast_BossBGM
  ;[1 1 1] Boss BGM
  (Audio|Components|Audio|SetSound (Variables|Default|GetBGM) "/Game/Sound/BGM/BGM_Boss0.BGM_Boss0")
  (Variables|Default|SetenterBoss true))

(event EventBeginPlay
  (bind _bgm (Variables|Default|GetBGM))
  ;[1 1 1] Event Begin Play
  (Variables|Default|SetcurMontage "/Game/Hunter/Blueprint/ActionMontage.ActionMontage")
  (Class|Hunter|SetHP 1e+02)
  (bind _returnvalue (Game|SpawnActorfromClass "/Game/Hunter/MouseCursor/BP_MouseCursor.BP_MouseCursor_C" (Transformation|GetActorTransform) "AlwaysSpawn" "OverrideRootScale" 0 0))
  (Variables|Default|SetMouseCursor _returnvalue)
  (bind _returnvalue_2 (Game|GetCurrentLevelName true))
  (if (Utilities|Enum|Equal(Enum) _returnvalue_2 "MyHome")
    (Audio|Components|Audio|SetSound _bgm "/Game/Sound/BGM/BGM_Lobby0.BGM_Lobby0")
    (else
      (Audio|Components|Audio|SetSound _bgm "/Game/Sound/BGM/BGM_Battle0.BGM_Battle0")))
  (Audio|Components|Audio|Play _bgm 0.0)
  (Variables|Default|SetreSpawnPos (Transformation|GetActorTransform))
  (Variables|Default|SetenterBoss false)
  (Variables|Default|SetRespawn false))

(event EventUpdateQuickSlot
  ;[1 1 1] Update Skill Slot
  (bind _aswbp_main_ui (Utilities|Casting|CastToWBP_MainUI (Variables|Default|GetMainUI)))
  (Default|UpdateQuickSlot _aswbp_main_ui))

(event EventUpdateSkillSlots
  ;[1 1 1] Update Skill Slot
  (bind _aswbp_main_ui (Utilities|Casting|CastToWBP_MainUI (Variables|Default|GetMainUI)))
  (Default|UpdateQuickSkill _aswbp_main_ui))

(event EventInteractEarthquake
  ;[1 1 1] Earthquake Interact
  (Camera|PlayWorldCameraShake "/Game/Hunter/Blueprint/BP_CameraShake.BP_CameraShake_C" (Transformation|GetWorldLocation (Variables|Default|GetFollowCamera)) 0.0 5e+02)
  (if (not (or (AI|Components|NavMovement|IsFalling (Variables|Character|GetCharacterMovement)) (Variables|Default|GetbInvincible)))
    (Character|LaunchCharacter "0.000000,0.000000,1000.000000" false false)))

(event EventEndPlay
  (params (EndPlayReason :type EEndPlayReason%20Enum :default "Destroyed"))
  ;[1 1 1] Save inventory Comp info -> base instance
  (bind _asbase_instance (Utilities|Casting|CastToBaseInstance (Game|GetGameInstance)))
  (Variables|/Script/PokeHunter.BaseInstance|SetInfoArray _asbase_instance (Variables|/Script/PokeHunter.InventoryComponent|GetInfoArray (Variables|Default|GetInventory))))

(event Game|Damage|EventRadialDamage
  (params (DamageReceived :type Float%20%28single-precision%29) (DamageType :type Damage%20Type%20Object%20Reference) (Origin :type Vector :default "0, 0, 0") (HitInfo :type Hit%20Result%20Structure%20%28by%20ref%29) (InstigatedBy :type Controller%20Object%20Reference) (DamageCauser :type Actor%20Object%20Reference))
  ;[1 1 1] Radial Damage Event
  (Character|LaunchCharacter (* (Math|Vector|Normalize (- (Transformation|GetActorLocation) Origin)) 1e+03) false false))

(event Input|ActionEvents|InputActionI_Key
  (params (Key :type Key%20Structure :default "None"))
  (bind _returnvalue (Pawn|GetController))
  ;[1 1 1] Open Inventory
  (:Pressed
    (bind _aswbp_main_ui (Utilities|Casting|CastToWBP_MainUI (Variables|Default|GetMainUI)))
    (if (Widget|IsVisible (Variables|/Game/UI/WBP_MainUI.WBP_MainUI_C|GetWBP_InventoryList _aswbp_main_ui))
      (Widget|SetVisibility (Variables|/Game/UI/WBP_MainUI.WBP_MainUI_C|GetWBP_InventoryList _aswbp_main_ui) "Hidden")
      (bind _as플레이어_컨트롤러 (Utilities|Casting|CastToPlayerController _returnvalue))
      (Input|SetInputModeGameOnly _as플레이어_컨트롤러 false)
      (Variables|/Script/Engine.PlayerController|SetbShowMouseCursor _as플레이어_컨트롤러 false)
      (Default|UpdateQuickSlot _aswbp_main_ui)
      (else
        (Default|InitializeInventory (Variables|/Game/UI/WBP_MainUI.WBP_MainUI_C|GetWBP_InventoryList _aswbp_main_ui))
        (Widget|SetVisibility (Variables|/Game/UI/WBP_MainUI.WBP_MainUI_C|GetWBP_InventoryList _aswbp_main_ui) "Visible")
        (bind _as플레이어_컨트롤러_2 (Utilities|Casting|CastToPlayerController _returnvalue))
        (Input|SetInputModeGameandUI _as플레이어_컨트롤러_2 0 "DoNotLock" true false)
        (Variables|/Script/Engine.PlayerController|SetbShowMouseCursor _as플레이어_컨트롤러_2 true)
        (Audio|PlaySound2D "/Game/Sound/SE/_O_popup_01._O_popup_01" 1.0 1.0 0.0 0 0)))))

(event Input|ActionEvents|InputActionBGM_Down
  (params (Key :type Key%20Structure :default "None"))
  ;[1 1 1] Control BGM
  (:Pressed
    (bind _output_get (Variables|Default|SetBGMVolume (- (Variables|Default|GetBGMVolume) 0.2)))
    (if (> _output_get 0.2)
      (Audio|Components|Audio|SetVolumeMultiplier (Variables|Default|GetBGM) (Variables|Default|GetBGMVolume) :!class /Script/Engine.AudioComponent)
      (else
        (bind _output_get_2 (Variables|Default|SetBGMVolume 0.2))
        (Audio|Components|Audio|SetVolumeMultiplier (Variables|Default|GetBGM) _output_get_2 :!class /Script/Engine.AudioComponent)))))

(event Input|ActionEvents|InputActionK_Key
  (params (Key :type Key%20Structure :default "None"))
  ;[1 1 1] Command Kill ALL
  (:Pressed
    (CallFunction|AllKillServer)))

(event Input|ActionEvents|InputActionP_Key
  (params (Key :type Key%20Structure :default "None"))
  ;[1 1 1] UI Pause
  (:Pressed
    (bind _aswbp_main_ui (Utilities|Casting|CastToWBP_MainUI (Variables|Default|GetMainUI)))
    (Widget|SetVisibility (Variables|/Game/UI/WBP_MainUI.WBP_MainUI_C|GetWBP_Pause_232 _aswbp_main_ui) "Visible")
    (bind _as플레이어_컨트롤러 (Utilities|Casting|CastToPlayerController (Pawn|GetController)))
    (Input|SetInputModeUIOnly _as플레이어_컨트롤러 (Variables|/Game/UI/WBP_MainUI.WBP_MainUI_C|GetWBP_Pause_232 _aswbp_main_ui) "DoNotLock" false)
    (Variables|/Script/Engine.PlayerController|SetbShowMouseCursor _as플레이어_컨트롤러 true)))

(event Input|ActionEvents|InputActionBGM_Up
  (params (Key :type Key%20Structure :default "None"))
  ;[1 1 1] Control BGM
  (:Pressed
    (bind _output_get (Variables|Default|SetBGMVolume (+ (Variables|Default|GetBGMVolume) 0.2)))
    (if (< _output_get 4.0)
      (Audio|Components|Audio|SetVolumeMultiplier (Variables|Default|GetBGM) (Variables|Default|GetBGMVolume) :!class /Script/Engine.AudioComponent)
      (else
        (bind _output_get_2 (Variables|Default|SetBGMVolume 4.0))
        (Audio|Components|Audio|SetVolumeMultiplier (Variables|Default|GetBGM) _output_get_2 :!class /Script/Engine.AudioComponent)))))

(event Input|MouseEvents|MouseWheelUp
  (params (Key :type Key%20Structure :default "None"))
  ;[1 1 1] Select Item
  (:Pressed
    (Variables|Default|SetCurQuickKey (+ (Variables|Default|GetCurQuickKey) 1))
    (Class|Hunter|ChangeQuickslot (Class|Actor|GetInputAxisKeyValue Key))
    (bind _aswbp_main_ui (Utilities|Casting|CastToWBP_MainUI (Variables|Default|GetMainUI)))
    (Default|UpdateQuickSlot _aswbp_main_ui)
    (Audio|PlaySound2D "/Game/Sound/SE/_O_quick_02._O_quick_02" 1.0 1.0 0.0 0 0)))

(event Input|MouseEvents|MouseWheelDown
  (params (Key :type Key%20Structure :default "None"))
  ;[1 1 1] Select Item
  (:Pressed
    (Variables|Default|SetCurQuickKey (- (Variables|Default|GetCurQuickKey) 1))
    (Class|Hunter|ChangeQuickslot (Class|Actor|GetInputAxisKeyValue Key))
    (bind _aswbp_main_ui (Utilities|Casting|CastToWBP_MainUI (Variables|Default|GetMainUI)))
    (Default|UpdateQuickSlot _aswbp_main_ui)
    (Audio|PlaySound2D "/Game/Sound/SE/_O_quick_02._O_quick_02" 1.0 1.0 0.0 0 0)))

(event Input|MouseEvents|Mouse2D
  (params (AxisValue :type Vector :default "0, 0, 0"))
  (bind _mousecursor (Variables|Default|GetMouseCursor))
  ;[1 1 1] 코멘트
  (if (Variables|Default|GetbPartnerMode)
    (bind _ashunter_controller (Utilities|Casting|CastToHunterController (Pawn|GetController)))
    (if (.ReturnValue (Game|Player|GetHitResultUnderCursorbyChannel _ashunter_controller "TraceTypeQuery3" false))
      (bind _asbp_mouse_cursor (Utilities|Casting|CastToBP_MouseCursor _mousecursor))
      (Default|OnVisible _asbp_mouse_cursor)
      (Transformation|SetWorldRotation (Variables|/Game/Hunter/MouseCursor/BP_MouseCursor.BP_MouseCursor_C|GetPlane _asbp_mouse_cursor) (Math|Rotator|MakeRotfromZ (.ImpactNormal (Collision|BreakHitResult (.HitResult (Game|Player|GetHitResultUnderCursorbyChannel _ashunter_controller "TraceTypeQuery3" false))))) false false)
      (Transformation|SetWorldLocation (Variables|/Script/Engine.Actor|GetRootComponent _asbp_mouse_cursor) (.Location (Collision|BreakHitResult (.HitResult (Game|Player|GetHitResultUnderCursorbyChannel _ashunter_controller "TraceTypeQuery3" false)))) false false)
      (bind _as플레이어_컨트롤러 (Utilities|Casting|CastToPlayerController (Pawn|GetController)))
      (if (Game|Player|IsInputKeyDown _as플레이어_컨트롤러 "LeftMouseButton")
        (Utilities|FlowControl|DoOnce false :!label _label
          (:Completed
            (Audio|PlaySound2D "/Game/Sound/SE/SFX_PetPing.SFX_PetPing" 2.0 1.0 0.0 0 0)))
        (else
          (goto _label Reset))))
    (else
      (bind _asbp_mouse_cursor_2 (Utilities|Casting|CastToBP_MouseCursor _mousecursor))
      (Default|OffVisible _asbp_mouse_cursor_2))))

(fn ConstructionScript)

(fn ReSpawnHunter
  (params (NewParam :type New%20Hunter%20Object%20Reference))
  (return))