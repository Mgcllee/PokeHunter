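; BP_DropItemBox is a dropped item box that pops upward with a sound when spawned and tumbles until it lands.
; BeginPlay applies an upward impulse to the physics-simulated mesh, and Tick spins it on roll and yaw.
; The first hit passes through ServerOnHit to MultiOnHit, which stops physics, ticking and RotatingMovement, then snaps actor and mesh to the hit point, aligned to the surface normal.
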(event OnComponentHit(StaticMesh)
  (params (HitComponent :type Primitive%20Component%20Object%20Reference) (OtherActor :type Actor%20Object%20Reference) (OtherComp :type Primitive%20Component%20Object%20Reference) (NormalImpulse :type Vector :default "0, 0, 0") (Hit :type Hit%20Result%20Structure%20%28by%20ref%29))
  (if (Physics|IsSimulatingPhysics (Variables|Default|GetStaticMesh) "None")
    (CallFunction|ServeronHit (.normal Hit) (.location Hit))))

(event Custom|MultiOnHit
  (params (Normal :type Vector) (LocVec :type Vector))
  (bind _staticmesh (Variables|Default|GetStaticMesh))
  (Physics|SetSimulatePhysics _staticmesh false)
  (Actor|Tick|SetActorTickEnabled false)
  (Transformation|SetRelativeRotation _staticmesh (Math|Rotator|MakeRotfromZX Normal (Transformation|GetActorForwardVector)) false false)
  (Transformation|SetWorldLocation (Variables|Default|GetStaticMesh) LocVec false false)
  (Transformation|SetActorLocation LocVec false false)
  (Components|Activation|Deactivate (Variables|Default|GetRotatingMovement)))

(event Custom|ServerOnHit
  (params (Normal :type Vector) (LocVec :type Vector))
  (CallFunction|MultionHit Normal LocVec))

(event EventBeginPlay
  (Audio|PlaySoundatLocation "/Game/Sound/SE/Item_drop0.Item_drop0" (Transformation|GetWorldLocation (Variables|Default|GetStaticMesh)) "0, 0, 0" 1.0 1.0 0.0 "/Game/Hunter/Blueprint/BP_PersonalSound.BP_PersonalSound" 0 0 0)
  (Physics|AddImpulse (Variables|Default|GetStaticMesh) "0.000000,0.000000,600.000000" "None" true))

(event Collision|EventActorBeginOverlap
  (params (OtherActor :type Actor%20Object%20Reference)))

(event EventTick
  (params (DeltaSeconds :type Float%20%28single-precision%29))
  (bind _returnvalue (* DeltaSeconds 8e+02))
  (Transformation|AddLocalRotation (Variables|Default|GetStaticMesh) (Math|Rotator|MakeRotator _returnvalue 0.0 _returnvalue) false false))

(event EventDestroyed
  (Audio|SpawnSoundatLocation 0 (Transformation|GetWorldLocation (Variables|Default|GetStaticMesh)) "0, 0, 0" 1.0 1.0 0.0 0 0))

(fn ConstructionScript)