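; BP_NewWolfPartner is a wolf partner actor with an ice spear attack and breath and storm collision volumes.
; BeginPlay disables both volumes, and the construction script scales the storm volume by StormSize.
; SetNiagaraSystem fires the detached spear Niagara effect toward the Target's location.
; ServerSpawnIceEffect relays to MultiSpawnIceEffect, which reattaches the spear to the capsule and spawns a hit effect at the Target; damage nodes are unwired.
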(event OnSystemFinished(SpearEffect)
  (params (PSystem :type Niagara%20Component%20Object%20Reference)))

(event Custom|SetNiagaraSystem
  (params (NewParam :type Niagara%20Component%20Object%20Reference))
  (bind _speareffect (Variables|Default|GetSpearEffect))
  (Components|Activation|Activate _speareffect true)
  (Effects|Components|ParticleSystem|SetVectorParameter _speareffect "TargetLoc" (Transformation|GetActorLocation (Variables|Default|GetTarget)))
  (Transformation|SetWorldRotation _speareffect "0, 0, 0" false false)
  (Transformation|DetachFromComponent _speareffect "KeepWorld" "KeepWorld" "KeepWorld" true)
  (Transformation|SetWorldTransform (Variables|Default|GetCapsuleComponent) (Transformation|GetActorTransform) false false))

(event Custom|CustomEvent
  (CallFunction|CustomEvent0))

(event Custom|CustomEvent_0
  (Variables|Default|SetbArriveParticle true))

(event Custom|ServerSpawnIceEffect
  (CallFunction|MultiSpawnIceEffect))

(event Custom|MultiSpawnIceEffect
  (Transformation|AttachComponentToComponent (Variables|Default|GetSpearEffect) (Variables|Default|GetCapsuleComponent) "None" "SnapToTarget" "SnapToTarget" "SnapToTarget" true)
  (Niagara|SpawnSystematLocation "/Game/VFXs/VFX_Spear/VFX_Spear_Hit.VFX_Spear_Hit" (Transformation|GetActorLocation (Variables|Default|GetTarget)))
  (CallFunction|CustomEvent))

(event EventBeginPlay
  (Collision|SetCollisionEnabled (Variables|Default|GetBreathCollision) "NoCollision")
  (Collision|SetCollisionEnabled (Variables|Default|GetStormCollision) "NoCollision"))

(event Collision|EventActorBeginOverlap
  (params (OtherActor :type Actor%20Object%20Reference)))

(fn ConstructionScript
  (bind _stormcollision (Variables|Default|GetStormCollision))
  (Transformation|SetRelativeScale3D _stormcollision (* (Variables|/Script/Engine.SceneComponent|GetRelativeScale3D _stormcollision) (Variables|Default|GetStormSize))))