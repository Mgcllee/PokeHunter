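; BP_EnemyController is a controller for the default enemy that queries its AI perception component.
; FindAgroActor gets hearing-perceived actors and returns whether the first one matches the enemy's AgroTarget, exiting the loop on that first element.
; Tick loops over sight-perceived actors with an empty body, and BeginPlay and the construction script do nothing.
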(event EventBeginPlay)

(event EventTick
  (params (DeltaSeconds :type Float%20%28single-precision%29))
  (for _array_element (Class|AIPerceptionComponent|GetPerceivedActors (Class|AIController|GetAIPerceptionComponent) "/Script/AIModule.AISense_Sight")
    _))

(fn ConstructionScript)

(fn FindAgroActor
  (bind _array_element (Utilities|Array|ForEachLoopwithBreak (Class|AIPerceptionComponent|GetPerceivedActors (Class|AIController|GetAIPerceptionComponent) "/Script/AIModule.AISense_Hearing"))
    (:LoopBody
      (return (== (Variables|/Script/PokeHunter.Enemy|GetAgroTarget (Variables|Default|GetEnemy)) _array_element)))))