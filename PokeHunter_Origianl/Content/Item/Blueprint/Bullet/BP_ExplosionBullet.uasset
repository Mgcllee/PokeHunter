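; Explosive bullet Blueprint that deals radial damage and plays a world camera shake through its ability event or when it hits a non-enemy.
; The ability event also enables the collision sphere, kept off from BeginPlay, and loops over overlapping Characters with an empty body.
; Knockback logic that would launch those Characters away from the blast is disconnected and never runs.
; Destruction plays the explosion sound at the mesh location.
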(event EventBeginPlay
  (Collision|SetCollisionEnabled (Variables|Default|GetSphere) "NoCollision"))

(event Collision|EventActorBeginOverlap
  (params (OtherActor :type Actor%20Object%20Reference)))

(event EventTick
  (params (DeltaSeconds :type Float%20%28single-precision%29)))

(event EventApplyAbillity
  (params (OtherActor :type Actor%20Object%20Reference) (OtherComponent :type Primitive%20Component%20Object%20Reference))
  (bind _staticmesh (Variables|Default|GetStaticMesh))
  (bind _returnvalue (Transformation|GetWorldLocation _staticmesh))
  (Collision|SetCollisionEnabled (Variables|Default|GetSphere) "QueryAndPhysics")
  (Game|Damage|ApplyRadialDamage 1e+01 _returnvalue 5e+02 "/Script/Engine.DamageType" 0 0 0 false "ECC_GameTraceChannel8")
  (Camera|PlayWorldCameraShake "/Game/Item/Blueprint/Bullet/BP_ExplosionCameraShake.BP_ExplosionCameraShake_C" _returnvalue 0.0 5e+03)
  (for _array_element (Collision|GetOverlappingActors (Variables|Default|GetSphere) "/Script/Engine.Character" :!class /Script/Engine.PrimitiveComponent)
    _))

(event EventOnHitNotEnemy
  (params (HitVec :type Vector%20%28by%20ref%29 :default "0, 0, 0"))
  (bind _staticmesh (Variables|Default|GetStaticMesh))
  (bind _returnvalue (Transformation|GetWorldLocation _staticmesh))
  (Game|Damage|ApplyRadialDamage 1e+01 _returnvalue 5e+02 "/Script/Engine.DamageType" 0 0 0 false "ECC_GameTraceChannel8")
  (Camera|PlayWorldCameraShake "/Game/Item/Blueprint/Bullet/BP_ExplosionCameraShake.BP_ExplosionCameraShake_C" _returnvalue 0.0 5e+03))

(event EventDestroyed
  (Audio|PlaySoundatLocation "/Game/Sound/Bullet/ExplosionBullet__2_.ExplosionBullet__2_" (Transformation|GetWorldLocation (Variables|Default|GetStaticMesh)) "0, 0, 0" 1.0 1.0 0.0 "/Game/Hunter/Blueprint/BP_PersonalSound.BP_PersonalSound" 0 0 0))

(fn ConstructionScript)