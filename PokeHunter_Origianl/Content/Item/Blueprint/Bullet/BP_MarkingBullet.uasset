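; BP_MarkingBullet is a bullet that marks an enemy as the partner target of the Hunter who owns it.
; ApplyAbillity sets that target on an Enemy, and destroys the bullet for other actors.
; A debug line trace from the mesh, ending at normalized velocity times 100 without the start offset, freezes and moves the bullet to any hit.
; The code attaching it to the enemy is disconnected.
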(event EventBeginPlay)

(event Collision|EventActorBeginOverlap
  (params (OtherActor :type Actor%20Object%20Reference)))

(event EventTick
  (params (DeltaSeconds :type Float%20%28single-precision%29)))

(event EventApplyAbillity
  (params (OtherActor :type Actor%20Object%20Reference) (OtherComponent :type Primitive%20Component%20Object%20Reference))
  (bind _staticmesh (Variables|Default|GetStaticMesh))
  (bind _staticmesh_2 (Variables|Default|GetStaticMesh))
  (bind _ashunter (Utilities|Casting|CastToHunter (Variables|Default|GetThisOwner)))
  (bind _asenemy (Utilities|Casting|CastToEnemy OtherActor)
    (:then
      (Class|Hunter|SetPartnerTarget _ashunter _asenemy)
      (bind (_outhit _returnvalue) (Class|KismetSystemLibrary|LineTraceSinglebyProfile (Transformation|GetSocketLocation _staticmesh_2 "None") (* (Math|Vector|Normalize (Transformation|GetComponentVelocity _staticmesh_2)) 1e+02) "Visibility" false 0 "ForDuration" true))
      (if _returnvalue
        (Development|PrintString (Utilities|GetDisplayName (.hitcomponent _outhit)))
        (Physics|SetSimulatePhysics _staticmesh false)
        (Collision|SetCollisionEnabled _staticmesh "NoCollision")
        (Transformation|SetActorLocation (.location _outhit) false false)))
    (:CastFailed
      (Actor|DestroyActor))))

(fn ConstructionScript)