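; BP_FireBullet is a fire bullet that passes a fire interaction to the actor it affects.
; Its ApplyAbillity event sends InteractFireMessage to the other actor along with the affected component.
; When destroyed, it plays an attenuated fireball sound at the mesh location.
; The Tick rotation of the mesh multiplies by zero, so it has no visible effect, and the hit handler is empty.
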(event OnComponentHit(StaticMesh)
  (params (HitComponent :type Primitive%20Component%20Object%20Reference) (OtherActor :type Actor%20Object%20Reference) (OtherComp :type Primitive%20Component%20Object%20Reference) (NormalImpulse :type Vector :default "0, 0, 0") (Hit :type Hit%20Result%20Structure%20%28by%20ref%29)))

(event EventBeginPlay)

(event Collision|EventActorBeginOverlap
  (params (OtherActor :type Actor%20Object%20Reference)))

(event EventTick
  (params (DeltaSeconds :type Float%20%28single-precision%29))
  (Transformation|AddLocalRotation (Variables|Default|GetStaticMesh) (Math|Rotator|MakeRotator (* (* DeltaSeconds 0.0) 0.0) (* (* DeltaSeconds 0.0) 0.0) 0.0) false false))

(event EventApplyAbillity
  (params (OtherActor :type Actor%20Object%20Reference) (OtherComponent :type Primitive%20Component%20Object%20Reference))
  (Class|ItemInteractInterface|InteractFire(Message) OtherActor OtherComponent))

(event EventDestroyed
  (Audio|PlaySoundatLocation "/Game/Sound/Bullet/Fireball+3__online-audio-converter_com_.Fireball+3__online-audio-converter_com_" (Transformation|GetWorldLocation (Variables|Default|GetStaticMesh)) "0, 0, 0" 1.0 1.0 0.0 "/Game/Hunter/Blueprint/BP_PersonalSound.BP_PersonalSound" 0 0 0))

(fn ConstructionScript)